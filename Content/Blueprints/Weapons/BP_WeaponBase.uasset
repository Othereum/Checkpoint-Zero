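; Base weapon Blueprint that supplies the animation and sound feedback for weapon events.
; Fire, deploy and reload events play montages for the weapon, the arms or both, with separate reload variants for an empty weapon.
; Cancelling a reload blends out both reload variants.
; Dry fire and firemode switches spawn sounds attached to the mesh.
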(event EventOnReloadCancelled
  (Class|Weapon|StopMontage 0.1 (Variables|Animation|GetReloadAnim) (Variables|Animation|GetArmsReloadAnim) 0)
  (Class|Weapon|StopMontage 0.1 (Variables|Animation|GetReloadAnim_Empty) (Variables|Animation|GetArmsReloadAnim_Empty) 0))

(event EventOnFire
  (Class|Weapon|PlayMontage (Variables|Animation|GetFireAnim) (Variables|Animation|GetArmsShootAnim)))

(event EventOnReloadStart
  (params (bEmpty :type Boolean))
  (Class|Weapon|PlayMontage (select bEmpty (Variables|Animation|GetReloadAnim_Empty) (Variables|Animation|GetReloadAnim)) (select bEmpty (Variables|Animation|GetArmsReloadAnim_Empty) (Variables|Animation|GetArmsReloadAnim))))

(event EventOnDryFire
  (Audio|SpawnSoundAttached (Variables|Default|GetTriggerSound) (Variables|Character|GetMesh) "None" "0, 0, 0" "0, 0, 0" "KeepRelativeOffset" false 1.0 1.0 0.0 0 0))

(event EventOnFiremodeSwitched
  (Audio|SpawnSoundAttached "/Game/Assets/Weapons/Sounds/SC_SwitchFiremode.SC_SwitchFiremode" (Variables|Character|GetMesh) "None" "0, 0, 0" "0, 0, 0" "KeepRelativeOffset" false 1.0 1.0 0.0 0 0))

(event EventOnDeploy
  (Class|Weapon|PlayMontage 0 (Variables|Animation|GetArmsDeployAnim)))

(fn ConstructionScript)