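; BP_SunSky drives a directional light as a geographically positioned sun with an advancing time of day.
; Tick advances SolarTime in hours, scaled by TimeSpeed and wrapped at 24, then calls UpdateSun, which the construction script also runs.
; UpdateSun converts SolarTime to hours, minutes and seconds, then feeds them with location, time zone and date into GetSunPosition.
; The resulting corrected elevation and azimuth set the light's pitch and yaw.
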(event EventTick
  (params (DeltaSeconds :type Float%20%28single-precision%29))
  (Variables|시간|SetSolarTime (Math|Float|%(Float) (+ (/ DeltaSeconds (/ 3.6e+03 (Variables|시간|GetTimeSpeed))) (Variables|시간|GetSolarTime)) 24.0))
  (CallFunction|UpdateSun))

(fn ConstructionScript
  (CallFunction|UpdateSun))

(fn UpdateSun
  (bind (_hour _minute _second) (CallFunction|GetHMSfromSolarTime (Variables|시간|GetSolarTime)))
  (bind _sunpositiondata (Class|SunPositionFunctionLibrary|GetSunPosition (Variables|Location|GetLatitude) (Variables|Location|GetLongitude) (Variables|Location|GetTimeZone) false (Variables|Date|GetYear) (Variables|Date|GetMonth) (Variables|Date|GetDay) _hour _minute _second))
  (Transformation|SetWorldRotation (Variables|Default|GetDirectionalLight) (Math|Rotator|MakeRotator 0.0 (.correctedelevation _sunpositiondata) (.azimuth _sunpositiondata)) false false))

(fn GetHMSfromSolarTime
  (params (SolarTime :type Float%20%28single-precision%29))
  (return (Math|Integer|%(Integer) (Math|Float|Truncate SolarTime) 24) (Math|Integer|%(Integer) (Math|Float|Truncate (* SolarTime 6e+01)) 60) (Math|Integer|%(Integer) (Math|Float|Truncate (* SolarTime 3.6e+03)) 60)))